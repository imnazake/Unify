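; Player character Blueprint that wires keyboard keys to Gameplay Container plugin inventory features.
; F sends a toggle-inventory gameplay event to itself when an active container component exists.
; E sphere-overlaps nearby world items and triggers a partial loot event for each through the ability system, targeting the controller's inventory.
; X pushes the item spawner widget onto the modal UI layer.
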(event Input|KeyboardEvents|F
  (params (Key :type Key%20Structure :default "None"))
  (:Pressed
    (Utilities|IsValid (Class|UnifyCharacter|GetActiveContainerComponent)
      (:Is%20Valid
        (Ability|SendGameplayEventtoActor self "(TagName=\"Input.ToggleInventory\")")))))

(event Input|KeyboardEvents|X
  (params (Key :type Key%20Structure :default "None"))
  ;[1 1 1] Gameplay Containers Plugin
  (:Pressed
    (|PushContenttoLayerforPlayer (.AsUnify%20Player%20Controller (Utilities|Casting|CastToUnifyPlayerController (Pawn|GetController))) "/GameplayContainers/UI/Tools/W_ItemSpawner.W_ItemSpawner_C" "(TagName=\"UI.Layer.Modals\")" true)))

(event Input|KeyboardEvents|E
  (params (Key :type Key%20Structure :default "None"))
  (bind _returnvalue (Pawn|GetController))
  (bind _returnvalue_2 (Class|GameplayContainerLibrary|GetInventoryComponentfromActor _returnvalue false))
  ;[1 1 1] Gameplay Container Plugin
  ; This might also run inside an ability blueprint
  (:Pressed
    (bind _outactors (Collision|SphereOverlapActors (Transformation|GetActorLocation) 2e+02 (Utilities|Array|MakeArray "ObjectTypeQuery2") "/GameplayContainers/Core/Entities/BP_WorldItem.BP_WorldItem_C" (Utilities|Array|MakeArray self)))
    (for _array_element _outactors
      (Class|GameplayContainerLibrary|TriggerLootItemEvent (Class|UnifyCharacter|GetUnifyAbilitySystemComponent) _array_element _returnvalue_2 (Class|GameplayContainerComponent|GetFirstSlotType _returnvalue_2) true))))

(fn ConstructionScript)